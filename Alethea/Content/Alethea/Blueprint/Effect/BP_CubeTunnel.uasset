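; BP_CubeTunnel is a trigger-box effect actor that runs the NS_CubeTunnel Niagara system while an actor overlaps it.
; On overlap it spawns the system at its own location, passing the box size and a line projected along the overlapping actor's forward vector, also drawn for debugging.
; Tick streams that actor's position into the effect, and leaving the box deactivates it.
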(event OnComponentBeginOverlap(Box)
  (params (OverlappedComponent :type Primitive%20Component%20Object%20Reference) (OtherActor :type Actor%20Object%20Reference) (OtherComp :type Primitive%20Component%20Object%20Reference) (OtherBodyIndex :type Integer) (bFromSweep :type Boolean) (SweepResult :type Hit%20Result%20Structure%20%28by%20ref%29))
  (bind _returnvalue (Transformation|GetActorForwardVector OtherActor))
  (bind _returnvalue_2 (Transformation|GetActorLocation OtherActor))
  (bind _returnvalue_3 (* _returnvalue 1.5e+03))
  (bind _returnvalue_4 (+ _returnvalue_2 _returnvalue_3))
  (if (Utilities|IsValid OtherActor)
    ;[1 1 1] debug
    (Rendering|Debug|DrawDebugLine _returnvalue_2 _returnvalue_4 "(R=1.000000,G=0.000000,B=0.000000,A=1.000000)" 0.5 1e+01)
    (bind _returnvalue_5 (Niagara|SpawnSystematLocation "/Game/Alethea/Effect/NiagaraSystem/NS_CubeTunnel.NS_CubeTunnel" (Transformation|GetActorLocation)))
    (if (Utilities|IsValid _returnvalue_5)
      (bind _output_get (Variables|Default|SetNiagara_Scene_Component _returnvalue_5))
      (Niagara|SetNiagaraVariable(Vector3) _output_get "Line Start" _returnvalue_2)
      (Niagara|SetNiagaraVariable(Vector3) (Variables|Default|GetNiagara_Scene_Component) "Line End" _returnvalue_4)
      (Niagara|SetNiagaraVariable(Vector3) (Variables|Default|GetNiagara_Scene_Component) "Box Size" (* (Variables|/Script/Engine.BoxComponent|GetBoxExtent (Variables|Default|GetBox)) 2.0)))))

(event OnComponentEndOverlap(Box)
  (params (OverlappedComponent :type Primitive%20Component%20Object%20Reference) (OtherActor :type Actor%20Object%20Reference) (OtherComp :type Primitive%20Component%20Object%20Reference) (OtherBodyIndex :type Integer))
  (if (Utilities|IsValid (Variables|Default|GetNiagara_Scene_Component))
    (Components|Activation|Deactivate (Variables|Default|GetNiagara_Scene_Component))
    (Utilities|FlowControl|Delay 0.2)))

(event EventBeginPlay)

(event Collision|EventActorBeginOverlap
  (params (OtherActor :type Actor%20Object%20Reference)))

(event EventTick
  (params (DeltaSeconds :type Float%20%28single-precision%29))
  (bind _niagara_scene_component (Variables|Default|GetNiagara_Scene_Component))
  (if (Utilities|IsValid _niagara_scene_component)
    (Niagara|SetNiagaraVariable(Vector3) _niagara_scene_component "PlayerPosition_Update" (Transformation|GetActorLocation (stale OnComponentBeginOverlap(Box) OtherActor)))))

(fn ConstructionScript)